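; Blueprint function library of shared helpers for debug printing, typed access to core gameplay objects, and timeline progress.
; Log functions print long-lasting on-screen messages in randomized colors, with the bool variant appending the value and tinting by true or false.
; Getters cast the game instance, game mode, and first player's controller and character to the project's Blueprint classes.
; A utility returns a timeline's playback position as a fraction of its length.
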(fn `GetGI`
  (returns (GI :type "/Game/ConcreteTemplate/Blueprints/BP_GameInstance Object Reference"))
  (bind _asbp_game_instance (cast `/Game/ConcreteTemplate/Blueprints/BP_GameInstance` (`GameplayStatics.GetGameInstance` null)))
  (return _asbp_game_instance))

(fn `GetGM`
  (returns (GM :type "/Game/ConcreteTemplate/Blueprints/BP_GameMode Object Reference"))
  (bind _asbp_game_mode (cast `/Game/ConcreteTemplate/Blueprints/BP_GameMode` (`GameplayStatics.GetGameMode` null)))
  (return _asbp_game_mode))

(fn `GetPChar`
  (returns (Char :type "/Game/ConcreteTemplate/Character/BP_Character Object Reference"))
  (return (cast `/Game/ConcreteTemplate/Character/BP_Character` (`GameplayStatics.GetPlayerCharacter` null) :!pure true)))

(fn `GetPCont`
  (returns (PCont :type "/Game/ConcreteTemplate/Blueprints/BP_PlayerController Object Reference"))
  (bind _asbp_player_controller (cast `/Game/ConcreteTemplate/Blueprints/BP_PlayerController` (`GameplayStatics.GetPlayerController` null)))
  (return _asbp_player_controller))

(fn `GetTimelinePercentage`
  (params (Timeline :type "TimelineComponent Object Reference"))
  (returns (`%` :type "Float (double-precision)"))
  (return (/ (`TimelineComponent.GetPlaybackPosition` Timeline) (`TimelineComponent.GetTimelineLength` Timeline))))

(fn `Log Erer`
  (params (String :type String))
  (`KismetSystemLibrary.PrintString` null String true true (make `LinearColor` (`KismetMathLibrary.RandomFloatInRange` 0.25 1.0) (`KismetMathLibrary.RandomFloatInRange` 0.25 1.0) (`KismetMathLibrary.RandomFloatInRange` 0.25 1.0) 1.0) 9999.0))

(fn `Log ErerBool`
  (params (String :type String) (Bool :type Boolean))
  (bind _returnvalue (`KismetMathLibrary.RandomFloatInRange` 0.0 0.8))
  (bind _returnvalue_2 (`KismetMathLibrary.RandomFloatInRange` 0.0 0.5))
  (`KismetSystemLibrary.PrintString` null (`KismetStringLibrary.Concat_StrStr` String " = " (select `bool` Bool :`false` "FALSE" :`true` "true")) true true (select `bool` Bool :`false` (make `LinearColor` 1.0 _returnvalue _returnvalue 1.0) :`true` (make `LinearColor` _returnvalue_2 1.0 _returnvalue_2 1.0)) 9999.0))

(fn `Log Ererror`
  (params (Error :type String))
  (bind _returnvalue (`KismetMathLibrary.RandomFloatInRange` 0.5 1.0))
  (`KismetSystemLibrary.PrintString` null Error true true (make `LinearColor` _returnvalue (`KismetMathLibrary.RandomFloatInRange` 0.0 0.5) _returnvalue 1.0) 9999.0))