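; Framed in-world web screen actor that swaps a blank screen for a browser widget while TriggerWebsite is overlapped.
; The EnableMouse volume shows a centred cursor and turns the player toward the actor, then restores game-only input on exit.
; The construction script scales the frame and gives BlankScreen and Cube dynamic materials with random colours and set emissive.
; DT_WebPages URL lookups feeding CallMediaPlayerManager are disconnected and never run.
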(event `self.ReceiveBeginPlay`
  (`SceneComponent.SetVisibility` (`self.BlankScreen`) true false)
  (`SceneComponent.SetVisibility` (`self.Widget`) false false))

(event `self.ReceiveTick`
  (params (DeltaSeconds :type "Float (single-precision)")))

(event `self.TriggerWebsite.OnComponentBeginOverlap`
  (params (OverlappedComponent :type "PrimitiveComponent Object Reference") (OtherActor :type "Actor Object Reference") (OtherComp :type "PrimitiveComponent Object Reference") (OtherBodyIndex :type Integer) (bFromSweep :type Boolean) (SweepResult :type "HitResult Structure (by ref)"))
  (`SceneComponent.SetVisibility` (`self.Widget`) true false)
  (`SceneComponent.SetVisibility` (`self.BlankScreen`) false false)
  (`/Engine/EditorBlueprintResources/StandardMacros.DoOnce` false))

(event `self.TriggerWebsite.OnComponentEndOverlap`
  (params (OverlappedComponent :type "PrimitiveComponent Object Reference") (OtherActor :type "Actor Object Reference") (OtherComp :type "PrimitiveComponent Object Reference") (OtherBodyIndex :type Integer))
  (`SceneComponent.SetVisibility` (`self.BlankScreen`) true false)
  (`SceneComponent.SetVisibility` (`self.Widget`) false false))

(event `self.EnableMouse.OnComponentBeginOverlap`
  (params (OverlappedComponent :type "PrimitiveComponent Object Reference") (OtherActor :type "Actor Object Reference") (OtherComp :type "PrimitiveComponent Object Reference") (OtherBodyIndex :type Integer) (bFromSweep :type Boolean) (SweepResult :type "HitResult Structure (by ref)"))
  (bind _returnvalue (`GameplayStatics.GetPlayerController` 0))
  (bind (_returnvalue_x _returnvalue_y) (`KismetMathLibrary.BreakVector2D` (`WidgetLayoutLibrary.GetViewportSize`)))
  (`|ExecutionSequence`
    (:`then_0`
      (bind _returnvalue_2 (`GameUserSettings.GetDefaultResolution`))
      (`PlayerController.SetMouseLocation` _returnvalue (/ (break `IntPoint` _returnvalue_2) 2) (/ (`.Y` (break `IntPoint` _returnvalue_2)) 2))
      (set `PlayerController.bShowMouseCursor` true _returnvalue)
      (set `PlayerController.bEnableClickEvents` false _returnvalue)
      (set `PlayerController.bEnableMouseOverEvents` false _returnvalue)
      ;[1 1 1] Set Player Rotation
      (bind _returnvalue_3 (`self.LookAtRotation` (`GameplayStatics.GetPlayerCharacter` 0) (`self.BlankScreen`)))
      (`Controller.SetControlRotation` (`GameplayStatics.GetPlayerController` 0) _returnvalue_3))
    (:`then_1`
      (`PlayerController.SetMouseLocation` _returnvalue (/ (`KismetMathLibrary.FTrunc` _returnvalue_x) 2) (/ (`KismetMathLibrary.FTrunc` _returnvalue_y) 2)))))

(event `self.EnableMouse.OnComponentEndOverlap`
  (params (OverlappedComponent :type "PrimitiveComponent Object Reference") (OtherActor :type "Actor Object Reference") (OtherComp :type "PrimitiveComponent Object Reference") (OtherBodyIndex :type Integer))
  (bind _returnvalue (`GameplayStatics.GetPlayerController` 0))
  (`WidgetBlueprintLibrary.SetInputMode_GameOnly` _returnvalue)
  (set `PlayerController.bShowMouseCursor` false _returnvalue)
  (set `PlayerController.bEnableClickEvents` false _returnvalue)
  (set `PlayerController.bEnableMouseOverEvents` false _returnvalue))

(fn `LookAtRotation`
  (params (MyActor :type "Actor Object Reference") (Target :type "ActorComponent Object Reference"))
  (returns (ReturnValue :type "Rotator Structure"))
  (return (`KismetMathLibrary.RInterpTo` (`self.K2_GetActorRotation` MyActor) (`KismetMathLibrary.MakeRotator` 0.0 (.pitch (`KismetMathLibrary.FindLookAtRotation` (`self.K2_GetActorLocation` MyActor) (`self.K2_GetActorLocation`))) (.yaw (`KismetMathLibrary.FindLookAtRotation` (`self.K2_GetActorLocation` MyActor) (`self.K2_GetActorLocation`)))) (`GameplayStatics.GetWorldDeltaSeconds`) 50.0)))

(fn `UserConstructionScript`
  (`PrimitiveComponent.CreateDynamicMaterialInstance` (`self.Frame`) 0 (`self.FrameMaterial`))
  (bind _output_get (set `self.FinalFrameScale` (* (`self.BaseFrameScale`) (`self.FrameScaleMult`))))
  (`SceneComponent.SetRelativeScale3D` (`self.Frame`) _output_get)
  (`PrimitiveComponent.SetMaterial` (`self.Widget`) 0 "/Game/Criee2018/Art/VideoStream/M_WebBrowser_Inst.M_WebBrowser_Inst")
  (bind _returnvalue (`PrimitiveComponent.CreateDynamicMaterialInstance` (`self.BlankScreen`) 0 "/Game/Criee2018/Art/VideoStream/M_WebBlankScreen_Inst.M_WebBlankScreen_Inst"))
  (bind _output_get_2 (set `self.ScreenMaterial` _returnvalue))
  (bind _returnvalue_2 (`PrimitiveComponent.CreateDynamicMaterialInstance` (`self.Cube`) 0 "/Game/Criee2018/Art/VideoStream/M_WebBlankScreen_Inst.M_WebBlankScreen_Inst"))
  (`MaterialInstanceDynamic.SetVectorParameterValue` _output_get_2 "Color" (make `LinearColor` (`KismetMathLibrary.RandomFloatInRange` 0.1 1.0) (`KismetMathLibrary.RandomFloatInRange` 0.1 1.0) (`KismetMathLibrary.RandomFloatInRange` 0.1 1.0) (`KismetMathLibrary.RandomFloatInRange` 0.5 1.0)))
  (`MaterialInstanceDynamic.SetVectorParameterValue` _returnvalue_2 "Color" (make `LinearColor` (`KismetMathLibrary.RandomFloatInRange` 0.1 1.0) (`KismetMathLibrary.RandomFloatInRange` 0.1 1.0) (`KismetMathLibrary.RandomFloatInRange` 0.1 1.0) (`KismetMathLibrary.RandomFloatInRange` 0.5 1.0)))
  (`MaterialInstanceDynamic.SetVectorParameterValue` _output_get_2 "Color_1" (make `LinearColor` (`KismetMathLibrary.RandomFloatInRange` 0.1 1.0) (`KismetMathLibrary.RandomFloatInRange` 0.1 1.0) (`KismetMathLibrary.RandomFloatInRange` 0.1 1.0) (`KismetMathLibrary.RandomFloatInRange` 0.5 1.0)))
  (`MaterialInstanceDynamic.SetVectorParameterValue` _returnvalue_2 "Color_1" (make `LinearColor` (`KismetMathLibrary.RandomFloatInRange` 0.1 1.0) (`KismetMathLibrary.RandomFloatInRange` 0.1 1.0) (`KismetMathLibrary.RandomFloatInRange` 0.1 1.0) (`KismetMathLibrary.RandomFloatInRange` 0.5 1.0)))
  (`MaterialInstanceDynamic.SetScalarParameterValue` _output_get_2 "Emissive" (`self.EmissiveValue`))
  (`MaterialInstanceDynamic.SetScalarParameterValue` _returnvalue_2 "Emissive" (`self.EmissiveValue`)))