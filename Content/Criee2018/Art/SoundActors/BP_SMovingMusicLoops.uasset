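; Sound actor that turns the Montecrypto lobby music into a granular texture with an audio-reactive cube, when Activate is set.
; A GranularSynth in scrub mode holds one note of long, unvaried grains while a looping timer jumps its playhead to random positions.
; An envelope follower on a source effect drives the cube's interpolated Z scale.
; Pressing P stops the synth.
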(event `Key|P`
  (params (Key :type "Key Structure"))
  (bind _granularsynth (`self.GranularSynth`))
  (:`Pressed`
    (`SynthComponent.Stop` _granularsynth)
    (`ActorComponent.Deactivate` _granularsynth)))

(event `self.ReceiveBeginPlay`
  (bind _granularsynth (`self.GranularSynth`))
  (bind _granularsynth_2 (`self.GranularSynth`))
  (if (`self.Activate`)
    (`GranularSynth.SetSoundWave` _granularsynth "/Game/Criee2018/Art/SoundWaves/MontecryptoLobbyMusicFinal.MontecryptoLobbyMusicFinal")
    (`ActorComponent.Activate` _granularsynth false)
    (`GranularSynth.SetPlaybackSpeed` _granularsynth 0.0)
    (`KismetSystemLibrary.K2_SetTimerDelegate` (delegate `Retrig`) 2.0 true)
    (`GranularSynth.SetGrainDuration` _granularsynth 2000.0 (0.0 0.0))
    (`GranularSynth.SetGrainsPerSecond` _granularsynth 1.0)
    (`GranularSynth.SetGrainPitch` _granularsynth 1.0 (0.0 0.0))
    (`SourceEffectEnvelopeFollowerPreset.RegisterEnvelopeFollowerListener` (`self.EnveloppeFollowerSourceEffectRef`) (`self.EnvelopeFollowerListener`))
    (`GranularSynth.SetScrubMode` _granularsynth_2 true)
    (`SynthComponent.Start` _granularsynth_2)
    (`GranularSynth.NoteOn` _granularsynth_2 64.0 127 -1.0)))

(event `Retrig`
  (bind _returnvalue (`KismetMathLibrary.RandomFloatInRange` 0.0 100.0))
  (`GranularSynth.SetPlayheadTime` (`self.GranularSynth`) _returnvalue 0.0 "FromBeginning")
  (`KismetSystemLibrary.PrintString` (`KismetStringLibrary.Conv_DoubleToString` _returnvalue)))

(event `self.EnvelopeFollowerListener.OnEnvelopeFollowerUpdate`
  (params (EnvelopeValue :type "Float (single-precision)"))
  (bind (_relativescale3d_x _relativescale3d_y _relativescale3d_z) (`KismetMathLibrary.BreakVector` (`SceneComponent.RelativeScale3D` (`self.Cube`))))
  (`SceneComponent.SetWorldScale3D` (`self.Cube`) (`KismetMathLibrary.MakeVector` _relativescale3d_x _relativescale3d_y (`KismetMathLibrary.FInterpTo` _relativescale3d_z (* 20.0 EnvelopeValue) (`GameplayStatics.GetWorldDeltaSeconds`) 10.0))))

(fn `UserConstructionScript`)